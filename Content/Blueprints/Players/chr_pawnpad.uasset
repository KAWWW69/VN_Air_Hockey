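; Player pawn for a paddle that is pushed around the horizontal plane by input axes labeled as mouse control.
; Forward_Backward and Left_Right scale their axis values by Speed and apply them as X and Y impulses to the Paddel component, so movement is physics-driven and mass-dependent.
; Two unconnected AddWorldOffset nodes remain in the graph and never run.
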(event Input|AxisEvents|InputAxisLeft_Right
  (params (AxisValue :type Float%20%28single-precision%29))
  ;[1 1 1] Movement Controller (Mouse)
  (Physics|AddImpulse (Variables|Default|GetPaddel) (Math|Vector|MakeVector 0.0 (* AxisValue (Variables|Default|GetSpeed)) 0.0) "None" false))

(event Input|AxisEvents|InputAxisForward_Backward
  (params (AxisValue :type Float%20%28single-precision%29))
  ;[1 1 1] Movement Controller (Mouse)
  (Physics|AddImpulse (Variables|Default|GetPaddel) (Math|Vector|MakeVector (* AxisValue (Variables|Default|GetSpeed)) 0.0 0.0) "None" false))

(fn ConstructionScript)